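; BP_BlackHole is a black hole actor with video-driven upper and lower disks that keeps turning toward the camera.
; On BeginPlay it opens and plays separate media sources on the upper and lower disk media players.
; Each Tick it points its X axis along the normalized direction to the player camera, billboard style, with a slight constant offset subtracted before normalizing.
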(event EventBeginPlay
  (bind _lowerdiskmedia (Variables|Default|GetLowerDiskMedia))
  (bind _upperdiskmedia (Variables|Default|GetUpperDiskMedia))
  (Media|MediaPlayer|OpenSource _lowerdiskmedia "/Game/BlackHole/Meshes/Black_Hole/Lower_Disk.Lower_Disk")
  (Media|MediaPlayer|Play _lowerdiskmedia :!class /Script/MediaAssets.MediaPlayer)
  (Media|MediaPlayer|OpenSource _upperdiskmedia "/Game/BlackHole/Meshes/Black_Hole/UpperDisk.UpperDisk")
  (Media|MediaPlayer|Play _upperdiskmedia :!class /Script/MediaAssets.MediaPlayer))

(event EventTick
  (params (DeltaSeconds :type Float%20%28single-precision%29))
  (Transformation|SetActorRotation (Math|Rotator|MakeRotfromX (Math|Vector|RotateVector (Math|Vector|Normalize (- (- (Transformation|GetActorLocation (Game|GetPlayerCameraManager 0)) (Transformation|GetActorLocation)) "1.000000,1.000000,1.000000")) "0, 0, 0"))))

(fn ConstructionScript)