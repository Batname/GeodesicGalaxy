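; Base orbit actor that carries a planet around a center point in the space scene.
; The construction script offsets the Planet child actor by the orbit radius.
; BeginPlay passes planet class, spin speed and axial tilt into the nested BP_PlanetBase, then scales it.
; While enabled, Tick yaws OrbitCenter by a fixed step each frame, so orbit speed depends on frame rate.
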(event EventBeginPlay
  (bind _asbp_planet_base (Utilities|Casting|CastToBP_PlanetBase (Variables|/Script/Engine.ChildActorComponent|GetChildActor (Variables|Default|GetPlanet))))
  (bind _output_get (Variables|/Game/GeodesicGalaxy/Blueprints/SpaceObjects/BP_PlanetBase.BP_PlanetBase_C|SetPlanetClass _asbp_planet_base (Variables|Default|GetPlanetClass)))
  (ChildActorComponent|SetChildActorClass (Variables|/Game/GeodesicGalaxy/Blueprints/SpaceObjects/BP_PlanetBase.BP_PlanetBase_C|GetChildActor _asbp_planet_base) _output_get)
  (Variables|/Game/GeodesicGalaxy/Blueprints/SpaceObjects/BP_PlanetBase.BP_PlanetBase_C|SetRotationSpeed _asbp_planet_base (Variables|Default|GetAxisSpeed))
  (Transformation|SetRelativeRotation (Variables|/Game/GeodesicGalaxy/Blueprints/SpaceObjects/BP_PlanetBase.BP_PlanetBase_C|GetPlanetAxis _asbp_planet_base) (Math|Rotator|MakeRotator 0.0 (Variables|Default|GetAxisRotOffset) 0.0) false false)
  (Transformation|SetRelativeScale3D (Variables|Default|GetPlanet) (Math|Conversions|ToVector(Float) (Variables|Default|GetScale))))

(event Collision|EventActorBeginOverlap
  (params (OtherActor :type Actor%20Object%20Reference)))

(event EventTick
  (params (DeltaSeconds :type Float%20%28single-precision%29))
  (if (Variables|Default|GetEnable)
    (Transformation|AddLocalRotation (Variables|Default|GetOrbitCenter) (Math|Rotator|MakeRotator 0.0 0.0 (Variables|Default|GetSpeed)) false false)))

(fn ConstructionScript
  (Transformation|SetRelativeLocation (Variables|Default|GetPlanet) (Math|Vector|MakeVector (Variables|Default|GetRadius) 0.0 0.0) false false))