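; Orbiting planet Blueprint that adds a configurable moon through a Moon child actor.
; On BeginPlay it casts that child actor to BP_Orbit_Planet_Base, sets its nested Planet child actor to MoonClass and copies the moon's scale, spin, axis tilt, orbit speed and radius onto it.
; The moon reuses the planet orbit Blueprint through nested child actors, and this graph runs no Tick logic of its own.
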(event EventBeginPlay
  (|CallParentFunction)
  (bind _asbp_orbit_planet_base (Utilities|Casting|CastToBP_Orbit_Planet_Base (Variables|/Script/Engine.ChildActorComponent|GetChildActor (Variables|Default|GetMoon))))
  (ChildActorComponent|SetChildActorClass (Variables|/Game/GeodesicGalaxy/Blueprints/SpaceObjects/BP_Orbit_Planet_Base.BP_Orbit_Planet_Base_C|GetPlanet _asbp_orbit_planet_base) (Variables|Default|GetMoonClass))
  (Variables|/Game/GeodesicGalaxy/Blueprints/SpaceObjects/BP_Orbit_Planet_Base.BP_Orbit_Planet_Base_C|SetScale _asbp_orbit_planet_base (Variables|Default|GetMoonScale))
  (Variables|/Game/GeodesicGalaxy/Blueprints/SpaceObjects/BP_Orbit_Planet_Base.BP_Orbit_Planet_Base_C|SetAxisSpeed _asbp_orbit_planet_base (Variables|Default|GetMoonAxisSpeed))
  (Variables|/Game/GeodesicGalaxy/Blueprints/SpaceObjects/BP_Orbit_Planet_Base.BP_Orbit_Planet_Base_C|SetSpeed _asbp_orbit_planet_base (Variables|Default|GetMoonOrbitSpeed))
  (Variables|/Game/GeodesicGalaxy/Blueprints/SpaceObjects/BP_Orbit_Planet_Base.BP_Orbit_Planet_Base_C|SetAxisRotOffset _asbp_orbit_planet_base (Variables|Default|GetMoonAxisAngle))
  (Variables|/Game/GeodesicGalaxy/Blueprints/SpaceObjects/BP_Orbit_Planet_Base.BP_Orbit_Planet_Base_C|SetRadius _asbp_orbit_planet_base (Variables|Default|GetMoonOrbitRadius)))

(event Collision|EventActorBeginOverlap
  (params (OtherActor :type Actor%20Object%20Reference))
  (|CallParentFunction OtherActor) ; This node is disabled and will not be called.\nDrag off pins to build functionality.
)

(event EventTick
  (params (DeltaSeconds :type Float%20%28single-precision%29))
  (|CallParentFunction DeltaSeconds) ; This node is disabled and will not be called.\nDrag off pins to build functionality.
)

(fn ConstructionScript
  (|CallParentFunction))