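; Base planet actor that displays a configurable planet class as a spinning child actor with a text label.
; The construction script and BeginPlay both assign PlanetClass to the child actor, and BeginPlay also pitches the PlanetAxis component by AxisAngle.
; Each tick adds RotationSpeed to the child's yaw without delta-time scaling, so spin depends on frame rate, and turns the text toward the player pawn.
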(event EventBeginPlay
  (ChildActorComponent|SetChildActorClass (Variables|Default|GetChildActor) (Variables|Default|GetPlanetClass))
  (CallFunction|SetAxisAngle))

(event Collision|EventActorBeginOverlap
  (params (OtherActor :type Actor%20Object%20Reference)))

(event EventTick
  (params (DeltaSeconds :type Float%20%28single-precision%29))
  (CallFunction|IncrementRotation)
  (CallFunction|RotatePlanet)
  (CallFunction|TextFacePawn))

(fn ConstructionScript
  (ChildActorComponent|SetChildActorClass (Variables|Default|GetChildActor) (Variables|Default|GetPlanetClass)))

(fn IncrementRotation
  (Variables|Default|SetRotationAngle (+ (Variables|Default|GetRotationAngle) (Variables|Default|GetRotationSpeed))))

(fn RotatePlanet
  (Transformation|SetRelativeRotation (Variables|Default|GetChildActor) (Math|Rotator|MakeRotator 0.0 0.0 (Variables|Default|GetRotationAngle)) false false))

(fn SetAxisAngle
  (Transformation|SetRelativeRotation (Variables|Default|GetPlanetAxis) (Math|Rotator|MakeRotator 0.0 (Variables|Default|GetAxisAngle) 0.0) false false))

(fn TextFacePawn
  (Transformation|SetWorldRotation (Variables|Default|GetTextRender) (Math|Rotator|FindLookatRotation (Transformation|GetWorldLocation (Variables|Default|GetTextRender)) (Transformation|GetActorLocation (Game|Player|GetPlayerPawn 0))) false false))