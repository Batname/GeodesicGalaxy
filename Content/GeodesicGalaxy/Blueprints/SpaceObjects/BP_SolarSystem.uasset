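; Solar system actor inside BP_Galaxy that animates the switch between Galaxy and System game states.
; Entering System, MoveTimeline slides the star system to the galaxy's MoveToLocation while shrinking the black hole and asteroids, then scales up everything except CenterPlanet.
; Returning reverses both stages: the Shrink timeline collapses the system before the move plays backward.
; DoOnce gates guard the transitions, which also toggle orbit planets and their trails.
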(event Custom|ResetScaleAnim
  (Utilities|FlowControl|DoOnce false) ; enters at Reset
)

(event Custom|ResetMove
  (bind _parent (Variables|Default|GetParent))
  (Utilities|FlowControl|DoOnce false) ; enters at Reset
)

(event Custom|ScaleAnimationEvent
  (Utilities|FlowControl|DoOnce false
    (:Completed
      (Variables|Default|SetMoveAnimating true)
      (if (Variables|Default|GetEnabled)
        (CallFunction|Deactivate)
        (bind (_direction _driver) (Timeline|Shrink PlayFromStart)
          (:Update
            (CallFunction|ScaleSystem (Math|Conversions|ToVector(Float) _driver))
            (Variables|Default|SetScaleDirection _direction))
          (:Finished
            (switch Utilities|FlowControl|Switch|SwitchonETimelineDirection (Variables|Default|GetScaleDirection)
              (:Forward
                (CallFunction|SystemReturn))
              (:Backward
                (CallFunction|Activate)))
            (Variables|Default|SetEnabled (not (Variables|Default|GetEnabled)))
            (CallFunction|ResetScaleAnim)))
        (else
          (Timeline|Shrink ReverseFromEnd))))))

(event Custom|SystemReturn
  (bind _parent (Variables|Default|GetParent))
  (bind _driver (Timeline|MoveTimeline ReverseFromEnd)
    (:Update
      (Transformation|SetRelativeLocation (Variables|/Game/GeodesicGalaxy/Blueprints/SpaceObjects/BP_Galaxy.BP_Galaxy_C|GetStarSystemChildActor (Variables|Default|GetParent)) (+ (Variables|Default|GetOriginLocation) (* (Variables|Default|GetDifferenceVector) _driver)) false false)
      (Transformation|SetRelativeScale3D (Variables|/Game/GeodesicGalaxy/Blueprints/SpaceObjects/BP_Galaxy.BP_Galaxy_C|GetBlackHoleChildActor _parent) (Math|Conversions|ToVector(Float) (* (- 1.0 _driver) 0.05)))
      (Transformation|SetRelativeScale3D (Variables|/Game/GeodesicGalaxy/Blueprints/SpaceObjects/BP_Galaxy.BP_Galaxy_C|GetAsteroidsChildActor _parent) (Math|Conversions|ToVector(Float) (* (- 1.0 _driver) 0.01))))
    (:Finished
      (switch Utilities|FlowControl|Switch|SwitchonEGameStage (Variables|Default|GetGameState)
        (:NewEnumerator0
          _)
        (:NewEnumerator1
          (CallFunction|ScaleAnimationEvent)))
      (CallFunction|ResetMove))))

(event EventBeginPlay
  (Input|EnableInput (Game|GetPlayerController 0))
  (bind _asbp_galaxy (Utilities|Casting|CastToBP_Galaxy (Actor|GetParentActor)))
  (Variables|Default|SetParent _asbp_galaxy)
  (Variables|Default|SetOriginLocation (Variables|/Script/Engine.SceneComponent|GetRelativeLocation (Variables|/Game/GeodesicGalaxy/Blueprints/SpaceObjects/BP_Galaxy.BP_Galaxy_C|GetStarSystemChildActor _asbp_galaxy)))
  (CallFunction|ScaleSystem (Math|Conversions|ToVector(Float) (select (Variables|Default|GetEnabled) (Math|Float|MakeLiteralFloat 1.0) 0.0))))

(event Collision|EventActorBeginOverlap
  (params (OtherActor :type Actor%20Object%20Reference)))

(event EventTick
  (params (DeltaSeconds :type Float%20%28single-precision%29)))

(event EventScaleAnimation)

(event EventGameStateChanged
  (params (GameState :type EGameStage%20Enum :default "NewEnumerator0"))
  (bind _parent (Variables|Default|GetParent))
  (bind _output_get (Variables|Default|SetGameState GameState))
  (Utilities|FlowControl|DoOnce false
    (:Completed
      (CallFunction|FindDiferenceVector)
      (switch Utilities|FlowControl|Switch|SwitchonEGameStage _output_get
        (:NewEnumerator0
          (CallFunction|ScaleAnimationEvent))
        (:NewEnumerator1
          (bind _driver (Timeline|MoveTimeline PlayFromStart)
            (:Update
              (Transformation|SetRelativeLocation (Variables|/Game/GeodesicGalaxy/Blueprints/SpaceObjects/BP_Galaxy.BP_Galaxy_C|GetStarSystemChildActor (Variables|Default|GetParent)) (+ (Variables|Default|GetOriginLocation) (* (Variables|Default|GetDifferenceVector) _driver)) false false)
              (Transformation|SetRelativeScale3D (Variables|/Game/GeodesicGalaxy/Blueprints/SpaceObjects/BP_Galaxy.BP_Galaxy_C|GetBlackHoleChildActor _parent) (Math|Conversions|ToVector(Float) (* (- 1.0 _driver) 0.05)))
              (Transformation|SetRelativeScale3D (Variables|/Game/GeodesicGalaxy/Blueprints/SpaceObjects/BP_Galaxy.BP_Galaxy_C|GetAsteroidsChildActor _parent) (Math|Conversions|ToVector(Float) (* (- 1.0 _driver) 0.01))))
            (:Finished
              (switch Utilities|FlowControl|Switch|SwitchonEGameStage (Variables|Default|GetGameState)
                (:NewEnumerator0
                  _)
                (:NewEnumerator1
                  (CallFunction|ScaleAnimationEvent)))
              (CallFunction|ResetMove))))))))

(event EventResetGalaxyPosition
  (params (NewParam :type EGameStage%20Enum :default "NewEnumerator0"))
  (if (Math|Vector|Equal(Vector) (Variables|Default|GetDifferenceVector) "0, 0, 0" 0.0001)
    (CallFunction|FindDiferenceVector))
  (Utilities|FlowControl|Delay 0.1)
  (switch Utilities|FlowControl|Switch|SwitchonEGameStage NewParam
    (:NewEnumerator0
      (Variables|Default|SetOriginLocation (Variables|/Script/Engine.SceneComponent|GetRelativeLocation (Variables|/Game/GeodesicGalaxy/Blueprints/SpaceObjects/BP_Galaxy.BP_Galaxy_C|GetStarSystemChildActor (Variables|Default|GetParent))))
      (CallFunction|FindDiferenceVector))
    (:NewEnumerator1
      (bind _output_get (Variables|Default|SetDestinationLocation (Variables|/Script/Engine.SceneComponent|GetRelativeLocation (Variables|/Game/GeodesicGalaxy/Blueprints/SpaceObjects/BP_Galaxy.BP_Galaxy_C|GetStarSystemChildActor (Variables|Default|GetParent)))))
      (Variables|Default|SetOriginLocation (- _output_get (Variables|Default|GetDifferenceVector))))))

(event Input|KeyboardEvents|SpaceBar
  (params (Key :type Key%20Structure))
  (:Pressed
    (CallFunction|ScaleAnimation)))

(fn ConstructionScript)

(fn ScaleSystem
  (params (NewScale3D :type Vector))
  (for _array_element (Components|GetChildrenComponents (Variables|Default|GetDefaultSceneRoot) false)
    (if (!= _array_element (Variables|Default|GetCenterPlanet))
      (Transformation|SetRelativeScale3D _array_element NewScale3D))))

(fn Activate
  (bind _outactors (Actor|GetAllActorsOfClass "/Game/GeodesicGalaxy/Blueprints/SpaceObjects/BP_Orbit_Planet_Base.BP_Orbit_Planet_Base_C"))
  (for _array_element _outactors
    (if (not (Variables|/Game/GeodesicGalaxy/Blueprints/SpaceObjects/BP_Orbit_Planet_Base.BP_Orbit_Planet_Base_C|GetEnable _array_element))
      (Components|Activation|SetActive (Variables|/Game/GeodesicGalaxy/Blueprints/SpaceObjects/BP_Orbit_Planet_Base.BP_Orbit_Planet_Base_C|GetTrail _array_element) false false)
      (Variables|/Game/GeodesicGalaxy/Blueprints/SpaceObjects/BP_Orbit_Planet_Base.BP_Orbit_Planet_Base_C|SetEnable _array_element true)
      (Development|PrintString "activate")))
  (return))

(fn Deactivate
  (bind _outactors (Actor|GetAllActorsOfClass "/Game/GeodesicGalaxy/Blueprints/SpaceObjects/BP_Orbit_Planet_Base.BP_Orbit_Planet_Base_C"))
  (for _array_element _outactors
    (Components|Activation|Deactivate (Variables|/Game/GeodesicGalaxy/Blueprints/SpaceObjects/BP_Orbit_Planet_Base.BP_Orbit_Planet_Base_C|GetTrail _array_element))
    (Variables|/Game/GeodesicGalaxy/Blueprints/SpaceObjects/BP_Orbit_Planet_Base.BP_Orbit_Planet_Base_C|SetEnable _array_element false)
    (Development|PrintString "deactivate"))
  (return))

(fn FindDiferenceVector
  (bind _outactors (Actor|GetAllActorsOfClass "/Game/GeodesicGalaxy/Blueprints/SpaceObjects/BP_Galaxy.BP_Galaxy_C"))
  (bind _output_get (Variables|Default|SetDestinationLocation (Variables|/Script/Engine.SceneComponent|GetRelativeLocation (Variables|/Game/GeodesicGalaxy/Blueprints/SpaceObjects/BP_Galaxy.BP_Galaxy_C|GetMoveToLocation (Utilities|Array|Get(acopy) _outactors)))))
  (Variables|Default|SetDifferenceVector (- _output_get (Variables|Default|GetOriginLocation))))