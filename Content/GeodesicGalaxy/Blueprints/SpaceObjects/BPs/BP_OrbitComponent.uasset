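; BP_OrbitComponent is a component that moves its owning actor around a looping path in the horizontal plane.
; Initialize stores center, radius, speed and enable flag, and prints the center.
; While enabled, Tick adds Speed to the angle each frame, independent of delta time, then sets the owner's location without sweeping.
; Cosine and sine multiply center plus radius, so the path circles world origin in XY at the center's height.
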(event Custom|Initialize
  (params (Center :type Vector) (Radius :type Float%20%28single-precision%29) (Speed :type Float%20%28single-precision%29) (Enable :type Boolean))
  (bind _output_get (Variables|Default|SetOrbitCenter Center))
  (Variables|Default|SetRadius Radius)
  (Variables|Default|SetSpeed Speed)
  (Variables|Default|SetEnable Enable)
  (Development|PrintString (Utilities|String|ToString(Vector) _output_get)))

(event Custom|IncrementAngle
  (Variables|Default|SetAngle (+ (Variables|Default|GetAngle) (Variables|Default|GetSpeed))))

(event EventBeginPlay)

(event EventTick
  (params (DeltaSeconds :type Float%20%28single-precision%29))
  (bind _orbitcenter (Variables|Default|GetOrbitCenter))
  (bind _radius (Variables|Default|GetRadius))
  (bind _angle (Variables|Default|GetAngle))
  (if (Variables|Default|GetEnable)
    (CallFunction|IncrementAngle)
    (Transformation|SetActorLocation (Components|GetOwner) (Math|Vector|MakeVector (* (+ (.x _orbitcenter) _radius) (Math|Trig|Cos(Degrees) _angle)) (* (+ (.y _orbitcenter) _radius) (Math|Trig|Sin(Degrees) _angle)) (.z _orbitcenter)) false false)))