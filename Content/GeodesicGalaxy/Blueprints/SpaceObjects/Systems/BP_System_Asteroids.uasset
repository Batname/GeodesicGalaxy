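; Asteroids system actor for the galaxy, a child Blueprint that sets up the asteroid field as one of the galaxy's switchable space systems.
; On BeginPlay it takes the galaxy's asteroids child actor as its base and origin location, and lists the star system and black hole child actors to hide.
; Pressing the 2 key prints a debug message and calls ActivateSystem to activate it.
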(event EventBeginPlay
  (bind _bp_galaxy (Variables|Default|GetBP_Galaxy))
  (bind _bp_galaxy_2 (Variables|Default|GetBP_Galaxy))
  (bind _childactorstohide (Variables|Default|GetChildActorsToHide))
  (bind _asteroidschildactor (Variables|/Game/GeodesicGalaxy/Blueprints/SpaceObjects/BP_Galaxy.BP_Galaxy_C|GetAsteroidsChildActor _bp_galaxy))
  (|CallParentFunction)
  (Utilities|Array|Clear (Variables|Default|GetChildActorsToHide))
  (Variables|Default|SetBaseChildActor _asteroidschildactor)
  (Variables|Default|SetOriginLocation (Variables|/Script/Engine.SceneComponent|GetRelativeLocation _asteroidschildactor))
  (Utilities|Array|Add _childactorstohide (Variables|/Game/GeodesicGalaxy/Blueprints/SpaceObjects/BP_Galaxy.BP_Galaxy_C|GetStarSystemChildActor _bp_galaxy_2))
  (Utilities|Array|Add _childactorstohide (Variables|/Game/GeodesicGalaxy/Blueprints/SpaceObjects/BP_Galaxy.BP_Galaxy_C|GetBlackHoleChildActor _bp_galaxy_2)))

(event Collision|EventActorBeginOverlap
  (params (OtherActor :type Actor%20Object%20Reference))
  (|CallParentFunction OtherActor) ; This node is disabled and will not be called.\nDrag off pins to build functionality.
)

(event EventTick
  (params (DeltaSeconds :type Float%20%28single-precision%29))
  (|CallParentFunction DeltaSeconds) ; This node is disabled and will not be called.\nDrag off pins to build functionality.
)

(event Input|KeyboardEvents|2
  (params (Key :type Key%20Structure))
  (:Pressed
    (Development|PrintString "asteroids  system activate")
    (CallFunction|ActivateSystem)))

(fn ConstructionScript
  (|CallParentFunction))