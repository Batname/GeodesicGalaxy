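; Star system variant of a galaxy space-object system, configuring inherited logic for switching between the galaxy and star system views.
; On BeginPlay it takes BPGalaxy's star system child actor as the base, saves its relative location as the origin, and registers the asteroids and black hole child actors to hide.
; Keys 1 and Q print debug text and call ActivateSystem and ResetToGalaxy respectively.
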(event EventBeginPlay
  (bind _bp_galaxy (Variables|Default|GetBP_Galaxy))
  (bind _childactorstohide (Variables|Default|GetChildActorsToHide))
  (bind _bp_galaxy_2 (Variables|Default|GetBP_Galaxy))
  (bind _starsystemchildactor (Variables|/Game/GeodesicGalaxy/Blueprints/SpaceObjects/BP_Galaxy.BP_Galaxy_C|GetStarSystemChildActor _bp_galaxy))
  (|CallParentFunction)
  (Utilities|Array|Clear (Variables|Default|GetChildActorsToHide))
  (Variables|Default|SetBaseChildActor _starsystemchildactor)
  (Variables|Default|SetOriginLocation (Variables|/Script/Engine.SceneComponent|GetRelativeLocation _starsystemchildactor))
  (Utilities|Array|Add _childactorstohide (Variables|/Game/GeodesicGalaxy/Blueprints/SpaceObjects/BP_Galaxy.BP_Galaxy_C|GetAsteroidsChildActor _bp_galaxy_2))
  (Utilities|Array|Add _childactorstohide (Variables|/Game/GeodesicGalaxy/Blueprints/SpaceObjects/BP_Galaxy.BP_Galaxy_C|GetBlackHoleChildActor _bp_galaxy_2)))

(event Collision|EventActorBeginOverlap
  (params (OtherActor :type Actor%20Object%20Reference))
  (|CallParentFunction OtherActor) ; This node is disabled and will not be called.\nDrag off pins to build functionality.
)

(event EventTick
  (params (DeltaSeconds :type Float%20%28single-precision%29))
  (|CallParentFunction DeltaSeconds) ; This node is disabled and will not be called.\nDrag off pins to build functionality.
)

(event Input|KeyboardEvents|1
  (params (Key :type Key%20Structure))
  (:Pressed
    (Development|PrintString "stat system activate")
    (CallFunction|ActivateSystem)))

(event Input|KeyboardEvents|Q
  (params (Key :type Key%20Structure))
  (:Pressed
    (Development|PrintString "reset to galaxy")
    (CallFunction|ResettoGalaxy)))

(fn ConstructionScript
  (|CallParentFunction))