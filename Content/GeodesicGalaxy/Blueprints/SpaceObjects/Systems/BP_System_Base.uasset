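; Base actor for a star system in the galaxy view, animating the transition between galaxy and system stages.
; Activation moves it to BP_Galaxy's target point while shrinking listed child actors, then scales up everything but the center planet.
; Returning replays both timelines in the opposite direction, then sets the XR player state to Galaxy.
; Planet orbits and trails are toggled on all BP_Orbit_Planet_Base actors in the level.
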(event Custom|ActivateSystem
  (bind _bp_xr_playerstate (Variables|Default|GetBP_XR_PlayerState))
  ;[1 1 1] Scale root of system
  (Variables|Default|SetbIsSystemActive true)
  (CallFunction|FindDiferenceVector)
  (bind (_direction _driver) (Timeline|MoveTimeline PlayFromStart)
    (:Update
      (Transformation|SetRelativeLocation (Variables|Default|GetBaseChildActor) (+ (Variables|Default|GetOriginLocation) (* (Variables|Default|GetDifferenceVector) _driver)) false false)
      (for _array_element (Variables|Default|GetChildActorsToHide)
        (switch Utilities|FlowControl|Switch|SwitchonETimelineDirection _direction
          (:Forward
            (if (> (Math|Vector|VectorLength (* (Transformation|GetWorldScale (.ChildActorComponent (Utilities|Struct|BreakFChildSystems _array_element))) (- 1.0 _driver))) 1e-05)
              (Transformation|SetWorldScale3D (.ChildActorComponent (Utilities|Struct|BreakFChildSystems _array_element)) (* (Transformation|GetWorldScale (.ChildActorComponent (Utilities|Struct|BreakFChildSystems _array_element))) (- 1.0 _driver)))))
          (:Backward
            (Transformation|SetWorldScale3D (.ChildActorComponent (Utilities|Struct|BreakFChildSystems _array_element)) (* (.OriginalWorldScale (Utilities|Struct|BreakFChildSystems _array_element)) (- 1.0 _driver)))))))
    (:Finished
      (if (Variables|Default|GetbIsSystemActive)
        (CallFunction|PlanetsScaleAnimationEvent)
        (else
          (Variables|/Game/GeodesicGalaxy/Blueprints/GameMode/BP_XR_PlayerState.BP_XR_PlayerState_C|SetEGameStage _bp_xr_playerstate "NewEnumerator0")
          (Default|CallChangeStateInterface _bp_xr_playerstate))))))

(event Custom|ResetToGalaxy
  ;[1 1 1] Scale root of system
  (Variables|Default|SetbIsSystemActive false)
  (CallFunction|PlanetsScaleAnimationEvent))

(event Custom|ResetPositionEvent
  (params (GameState :type EGameStage%20Enum :default "NewEnumerator0"))
  ;[1 1 1] RE Position
  (if (Math|Vector|Equal(Vector) (Variables|Default|GetDifferenceVector) "0, 0, 0" 0.0001)
    (CallFunction|FindDiferenceVector))
  (switch Utilities|FlowControl|Switch|SwitchonEGameStage GameState
    (:NewEnumerator0
      (Variables|Default|SetOriginLocation (Variables|/Script/Engine.SceneComponent|GetRelativeLocation (Variables|Default|GetBaseChildActor)))
      (CallFunction|FindDiferenceVector))
    (:NewEnumerator1
      (bind _output_get (Variables|Default|SetDestinationLocation (Variables|/Script/Engine.SceneComponent|GetRelativeLocation (Variables|Default|GetBaseChildActor))))
      (Variables|Default|SetOriginLocation (- _output_get (Variables|Default|GetDifferenceVector))))))

(event Custom|PlanetsScaleAnimationEvent
  ;[1 1 1] Scale Planets
  (Variables|Default|SetMoveAnimating true)
  (if (Variables|Default|GetPlanetsEnabled)
    (CallFunction|Deactivate)
    (bind (_direction _driver) (Timeline|Shrink PlayFromStart)
      (:Update
        (CallFunction|ScaleSystem (Math|Conversions|ToVector(Float) _driver))
        (Variables|Default|SetTimelineScaleDirection _direction))
      (:Finished
        (switch Utilities|FlowControl|Switch|SwitchonETimelineDirection (Variables|Default|GetTimelineScaleDirection)
          (:Forward
            (CallFunction|SystemReturn))
          (:Backward
            (CallFunction|Activate)))
        (Variables|Default|SetPlanetsEnabled (not (Variables|Default|GetPlanetsEnabled)))))
    (else
      (Timeline|Shrink ReverseFromEnd))))

(event Custom|SystemReturn
  (bind _bp_xr_playerstate (Variables|Default|GetBP_XR_PlayerState))
  ;[1 1 1] Scale root of system
  (bind (_direction _driver) (Timeline|MoveTimeline ReverseFromEnd)
    (:Update
      (Transformation|SetRelativeLocation (Variables|Default|GetBaseChildActor) (+ (Variables|Default|GetOriginLocation) (* (Variables|Default|GetDifferenceVector) _driver)) false false)
      (for _array_element (Variables|Default|GetChildActorsToHide)
        (switch Utilities|FlowControl|Switch|SwitchonETimelineDirection _direction
          (:Forward
            (if (> (Math|Vector|VectorLength (* (Transformation|GetWorldScale (.ChildActorComponent (Utilities|Struct|BreakFChildSystems _array_element))) (- 1.0 _driver))) 1e-05)
              (Transformation|SetWorldScale3D (.ChildActorComponent (Utilities|Struct|BreakFChildSystems _array_element)) (* (Transformation|GetWorldScale (.ChildActorComponent (Utilities|Struct|BreakFChildSystems _array_element))) (- 1.0 _driver)))))
          (:Backward
            (Transformation|SetWorldScale3D (.ChildActorComponent (Utilities|Struct|BreakFChildSystems _array_element)) (* (.OriginalWorldScale (Utilities|Struct|BreakFChildSystems _array_element)) (- 1.0 _driver)))))))
    (:Finished
      (if (Variables|Default|GetbIsSystemActive)
        (CallFunction|PlanetsScaleAnimationEvent)
        (else
          (Variables|/Game/GeodesicGalaxy/Blueprints/GameMode/BP_XR_PlayerState.BP_XR_PlayerState_C|SetEGameStage _bp_xr_playerstate "NewEnumerator0")
          (Default|CallChangeStateInterface _bp_xr_playerstate))))))

(event EventBeginPlay
  ;[1 1 1] Begin Play
  (Utilities|FlowControl|Sequence
    (:then_0
      (Input|EnableInput (Game|GetPlayerController 0))
      (bind _asbp_galaxy (Utilities|Casting|CastToBP_Galaxy (Actor|GetParentActor)))
      (Variables|Default|SetBP_Galaxy _asbp_galaxy)
      (bind _asbp_xr_player_state (Utilities|Casting|CastToBP_XR_PlayerState (Variables|/Script/Engine.Pawn|GetPlayerState (Game|Player|GetPlayerPawn 0))))
      (Variables|Default|SetBP_XR_PlayerState _asbp_xr_player_state))
    (:then_1
      (CallFunction|ScaleSystem (Math|Conversions|ToVector(Float) (select (Variables|Default|GetPlanetsEnabled) (Math|Float|MakeLiteralFloat 1.0) 0.0))))))

(fn ConstructionScript)

(fn ScaleSystem
  (params (NewScale3D :type Vector))
  (for _array_element (Components|GetChildrenComponents (Variables|Default|GetDefaultSceneRoot) false)
    (if (!= _array_element (Variables|Default|GetCenterPlanet))
      (Transformation|SetRelativeScale3D _array_element NewScale3D))))

(fn Activate
  (bind _outactors (Actor|GetAllActorsOfClass "/Game/GeodesicGalaxy/Blueprints/SpaceObjects/Planet/BP_Orbit_Planet_Base.BP_Orbit_Planet_Base_C"))
  (for _array_element _outactors
    (if (not (Variables|/Game/GeodesicGalaxy/Blueprints/SpaceObjects/Planet/BP_Orbit_Planet_Base.BP_Orbit_Planet_Base_C|GetEnable _array_element))
      (Components|Activation|SetActive (Variables|/Game/GeodesicGalaxy/Blueprints/SpaceObjects/Planet/BP_Orbit_Planet_Base.BP_Orbit_Planet_Base_C|GetTrail _array_element) false false)
      (Variables|/Game/GeodesicGalaxy/Blueprints/SpaceObjects/Planet/BP_Orbit_Planet_Base.BP_Orbit_Planet_Base_C|SetEnable _array_element true)))
  (return))

(fn Deactivate
  (bind _outactors (Actor|GetAllActorsOfClass "/Game/GeodesicGalaxy/Blueprints/SpaceObjects/Planet/BP_Orbit_Planet_Base.BP_Orbit_Planet_Base_C"))
  (for _array_element _outactors
    (Components|Activation|Deactivate (Variables|/Game/GeodesicGalaxy/Blueprints/SpaceObjects/Planet/BP_Orbit_Planet_Base.BP_Orbit_Planet_Base_C|GetTrail _array_element))
    (Variables|/Game/GeodesicGalaxy/Blueprints/SpaceObjects/Planet/BP_Orbit_Planet_Base.BP_Orbit_Planet_Base_C|SetEnable _array_element false))
  (return))

(fn FindDiferenceVector
  (bind _outactors (Actor|GetAllActorsOfClass "/Game/GeodesicGalaxy/Blueprints/SpaceObjects/BP_Galaxy.BP_Galaxy_C"))
  (bind _output_get (Variables|Default|SetDestinationLocation (Variables|/Script/Engine.SceneComponent|GetRelativeLocation (Variables|/Game/GeodesicGalaxy/Blueprints/SpaceObjects/BP_Galaxy.BP_Galaxy_C|GetMoveToLocation (Utilities|Array|Get(acopy) _outactors)))))
  (Variables|Default|SetDifferenceVector (- _output_get (Variables|Default|GetOriginLocation))))