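; Black hole system in the geodesic galaxy, a child system Blueprint activated with key 3 and reset to the galaxy with E.
; On BeginPlay it registers its galaxy child actor as the base and lists the asteroid and star system actors for hiding.
; Its planet-scale override uses one timeline, forward and reversed, to scale the center body relative to its original size.
; Forward completion changes the XR player game stage; backward completion runs the system return.
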(event EventBeginPlay
  (bind _bp_galaxy (Variables|Default|GetBP_Galaxy))
  (bind _bp_galaxy_2 (Variables|Default|GetBP_Galaxy))
  (bind _bp_galaxy_3 (Variables|Default|GetBP_Galaxy))
  (bind _starsystemchildactor (Variables|/Game/GeodesicGalaxy/Blueprints/SpaceObjects/BP_Galaxy.BP_Galaxy_C|GetStarSystemChildActor _bp_galaxy_3))
  (bind _asteroidschildactor (Variables|/Game/GeodesicGalaxy/Blueprints/SpaceObjects/BP_Galaxy.BP_Galaxy_C|GetAsteroidsChildActor _bp_galaxy_2))
  (bind _blackholechildactor (Variables|/Game/GeodesicGalaxy/Blueprints/SpaceObjects/BP_Galaxy.BP_Galaxy_C|GetBlackHoleChildActor _bp_galaxy))
  (|CallParentFunction)
  (Utilities|FlowControl|Sequence
    (:then_0
      (Utilities|Array|Clear (Variables|Default|GetChildActorsToHide))
      (Variables|Default|SetBaseChildActor _blackholechildactor)
      (Variables|Default|SetOriginLocation (Variables|/Script/Engine.SceneComponent|GetRelativeLocation _blackholechildactor))
      (Utilities|Array|Add (Variables|Default|GetChildActorsToHide) (Utilities|Struct|MakeFChildSystems _asteroidschildactor (Transformation|GetWorldScale _asteroidschildactor)))
      (Utilities|Array|Add (Variables|Default|GetChildActorsToHide) (Utilities|Struct|MakeFChildSystems _starsystemchildactor (Transformation|GetWorldScale _starsystemchildactor))))
    (:then_1
      (Variables|Default|SetBlackHoleOriginalScale (Transformation|GetWorldScale (Variables|Default|GetCenterPlanet))))))

(event EventPlanetsScaleAnimationEvent
  (bind _bp_xr_playerstate (Variables|Default|GetBP_XR_PlayerState))
  ;[1 1 1] Scale Planets - Override
  (if (Variables|Default|GetbIsSystemActive)
    (bind (_direction _driver) (Timeline|Shrink_child PlayFromStart)
      (:Update
        (bind _output_get (Variables|Default|SetTimelineScaleDirection _direction))
        (switch Utilities|FlowControl|Switch|SwitchonETimelineDirection _output_get
          (:Forward
            (Transformation|SetWorldScale3D (Variables|Default|GetCenterPlanet) (+ (* (Variables|Default|GetBlackHoleOriginalScale) (* (- 1.0 _driver) (Variables|Default|GetBlackHoleScalar))) (Variables|Default|GetBlackHoleOriginalScale))))
          (:Backward
            (Transformation|SetWorldScale3D (Variables|Default|GetCenterPlanet) (+ (* (Variables|Default|GetBlackHoleScaleValue) (- 1.0 _driver)) (Variables|Default|GetBlackHoleOriginalScale))))))
      (:Finished
        (Variables|Default|SetBlackHoleScaleValue (- (Transformation|GetWorldScale (Variables|Default|GetCenterPlanet)) (Variables|Default|GetBlackHoleOriginalScale)))
        (switch Utilities|FlowControl|Switch|SwitchonETimelineDirection (Variables|Default|GetTimelineScaleDirection)
          (:Forward
            (Variables|/Game/GeodesicGalaxy/Blueprints/GameMode/BP_XR_PlayerState.BP_XR_PlayerState_C|SetEGameStage _bp_xr_playerstate "NewEnumerator1")
            (Default|CallChangeStateInterface _bp_xr_playerstate))
          (:Backward
            (CallFunction|SystemReturn)))))
    (else
      (Timeline|Shrink_child ReverseFromEnd))))

(event EventTick
  (params (DeltaSeconds :type Float%20%28single-precision%29))
  (|CallParentFunction DeltaSeconds))

(event Collision|EventActorBeginOverlap
  (params (OtherActor :type Actor%20Object%20Reference))
  (|CallParentFunction OtherActor))

(event Input|KeyboardEvents|3
  (params (Key :type Key%20Structure))
  (:Pressed
    (CallFunction|ActivateSystem)))

(event Input|KeyboardEvents|E
  (params (Key :type Key%20Structure))
  (:Pressed
    (CallFunction|ResettoGalaxy)))

(fn ConstructionScript
  (|CallParentFunction))