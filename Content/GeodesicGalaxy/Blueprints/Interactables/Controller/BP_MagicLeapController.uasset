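; Magic Leap controller actor for Geodesic Galaxy that projects a pointing beam and tracks which BP_System it aims at.
; Each tick it resets the beam, hit sphere and target references, then line traces along the beam's forward vector on the Visibility channel.
; A hit shortens the spline-mesh beam, shows the sphere at the impact point and stores the hit actor's parent as PointingSystem if it is a BP_System.
; ToggleMenu sets the controller's visibility.
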(event EventBeginPlay
  (bind _beamsplinemesh (Variables|Default|GetBeamSplineMesh))
  (Variables|Default|SetInitialBeamEndPosition (SplineMesh|GetEndPosition _beamsplinemesh))
  (Variables|Default|SetInitialBeamTangent (SplineMesh|GetEndTangent _beamsplinemesh))
  (Development|SetHiddeninGame (Variables|Default|GetCollisionSphere) true false))

(event EventToggleMenu
  (params (bIsHidden :type Boolean))
  (Development|SetHiddeninGame (Variables|Default|GetMagicLeapController) bIsHidden true))

(event EventTick
  (params (DeltaSeconds :type Float%20%28single-precision%29))
  (bind _collisionsphere (Variables|Default|GetCollisionSphere))
  (bind _beamsplinemesh (Variables|Default|GetBeamSplineMesh))
  (bind _beamsplinemesh_2 (Variables|Default|GetBeamSplineMesh))
  (bind _returnvalue (Transformation|GetWorldLocation _beamsplinemesh))
  (CallFunction|ResetCollisionVisual)
  (bind (_outhit _returnvalue_2) (Collision|LineTraceByChannel _returnvalue (+ _returnvalue (* (Math|Vector|GetForwardVector (Transformation|GetWorldRotation _beamsplinemesh)) (Math|Vector|VectorLength (SplineMesh|GetEndPosition (Variables|Default|GetBeamSplineMesh))))) "TraceTypeQuery1" false 0 "None"))
  (if _returnvalue_2
    (SplineMesh|SetEndPosition _beamsplinemesh_2 (Math|Vector|MakeVector (Math|Vector|VectorLength (- (.Location (Collision|BreakHitResult _outhit)) (Transformation|GetWorldLocation (Variables|Default|GetBeamSplineMesh)))) 0.0 0.0) true)
    (SplineMesh|SetEndTangent _beamsplinemesh_2 (Math|Vector|MakeVector (Math|Vector|VectorLength (- (.Location (Collision|BreakHitResult _outhit)) (Transformation|GetWorldLocation (Variables|Default|GetBeamSplineMesh)))) 0.0 0.0) true :!class /Script/Engine.SplineMeshComponent)
    (Transformation|SetWorldLocation _collisionsphere (.ImpactPoint (Collision|BreakHitResult _outhit)) false false)
    (Development|SetHiddeninGame _collisionsphere false false)
    (Utilities|IsValid (Actor|GetParentActor (.HitActor (Collision|BreakHitResult _outhit)))
      (:Is%20Valid
        (bind _asbp_system (Utilities|Casting|CastToBP_System (Actor|GetParentActor (.HitActor (Collision|BreakHitResult _outhit)))))
        (Variables|Default|SetPointingSystem _asbp_system)))))

(fn ConstructionScript)

(fn ResetCollisionVisual
  ;[1 1 1] Reset
  (SplineMesh|SetEndPosition (Variables|Default|GetBeamSplineMesh) (Variables|Default|GetInitialBeamEndPosition) true)
  (SplineMesh|SetEndTangent (Variables|Default|GetBeamSplineMesh) (Variables|Default|GetInitialBeamEndPosition) true :!class /Script/Engine.SplineMeshComponent)
  (Development|SetHiddeninGame (Variables|Default|GetCollisionSphere) true false)
  (Variables|Default|SetPointingSystem 0)
  (Variables|Default|SetBP_PlanetBase 0))