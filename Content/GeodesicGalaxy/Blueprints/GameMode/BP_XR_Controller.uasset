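; Player controller for Geodesic Galaxy that turns Magic Leap controller input into gameplay messages.
; Each input finds all actors implementing BPI_CoreInterface and broadcasts to them, avoiding direct references.
; Bumper resets galaxy position using the game stage from BP_XR_PlayerState, Home sends go-back, and a positive trigger axis forwards its value.
; The trigger press action only prints a debug string.
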(event EventBeginPlay)

(event Input|ActionEvents|InputActionLeapHomeAction
  (params (Key :type Key%20Structure))
  (:Pressed
    (bind _outactors (Actor|GetAllActorswithInterface "/Game/GeodesicGalaxy/Blueprints/Core/BPI_CoreInterface.BPI_CoreInterface_C"))
    (for _array_element _outactors
      (Class|BPICoreInterface|GoBackAction(Message) _array_element))))

(event Input|ActionEvents|InputActionLeapBumperAction
  (params (Key :type Key%20Structure))
  (:Pressed
    (bind _outactors (Actor|GetAllActorswithInterface "/Game/GeodesicGalaxy/Blueprints/Core/BPI_CoreInterface.BPI_CoreInterface_C"))
    (for _array_element _outactors
      (bind _asbp_xr_player_state (Utilities|Casting|CastToBP_XR_PlayerState (Variables|GetPlayerState)))
      (Class|BPICoreInterface|ResetGalaxyPosition(Message) _array_element (Variables|/Game/GeodesicGalaxy/Blueprints/GameMode/BP_XR_PlayerState.BP_XR_PlayerState_C|GetEGameStage _asbp_xr_player_state)))))

(event Input|ActionEvents|InputActionLeapTriggerAction
  (params (Key :type Key%20Structure))
  (:Pressed
    (Development|PrintString "TriggerAction")))

(event Input|AxisEvents|InputAxisLeapTriggerAxis
  (params (AxisValue :type Float%20%28single-precision%29))
  (if (> AxisValue 0.0)
    (bind _outactors (Actor|GetAllActorswithInterface "/Game/GeodesicGalaxy/Blueprints/Core/BPI_CoreInterface.BPI_CoreInterface_C"))
    (for _array_element _outactors
      (Class|BPICoreInterface|TriggerAction(Message) _array_element AxisValue))))

(fn ConstructionScript)