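; BP_XR_PlayerState is the XR player state that drives game stages, entering the Galaxy stage on BeginPlay.
; ProcessGameStage stores the stage, runs its handler (only Galaxy is implemented), then broadcasts the change to every actor implementing BPI_CoreInterface.
; The Galaxy handler spawns a BP_Galaxy a set distance along the player camera's forward vector, but only if none exists yet.
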(event EventBeginPlay
  (CallFunction|ProcessGameStage "NewEnumerator0"))

(fn ConstructionScript)

(fn ProcessGameStage
  (params (EGameStage :type EGameStage%20Enum :default "NewEnumerator0"))
  (Variables|Default|SetEGameStage EGameStage)
  (Utilities|FlowControl|Sequence
    (:then_0
      (switch Utilities|FlowControl|Switch|SwitchonEGameStage (Variables|Default|GetEGameStage)
        (:NewEnumerator0
          (CallFunction|ProcessGalaxyStage))))
    (:then_1
      (bind _outactors (Actor|GetAllActorswithInterface "/Game/GeodesicGalaxy/Blueprints/Core/BPI_CoreInterface.BPI_CoreInterface_C"))
      (for _array_element _outactors
        (Class|BPICoreInterface|GameStateChanged(Message) _array_element (Variables|Default|GetEGameStage))))))

(fn ProcessGalaxyStage
  (bind _returnvalue (Game|GetPlayerCameraManager 0))
  (Utilities|FlowControl|Sequence
    (:then_0
      (bind _outactors (Actor|GetAllActorsOfClass "/Game/GeodesicGalaxy/Blueprints/SpaceObjects/BP_Galaxy.BP_Galaxy_C"))
      (if (not (Math|Conversions|ToBoolean(Integer) (Utilities|Array|Length _outactors)))
        (Game|SpawnActorfromClass "/Game/GeodesicGalaxy/Blueprints/SpaceObjects/BP_Galaxy.BP_Galaxy_C" (Math|Transform|MakeTransform (+ (Transformation|GetActorLocation _returnvalue) (* (Math|Vector|GetForwardVector (Transformation|GetActorRotation _returnvalue)) (Variables|Default|GetSpawnGalaxyDistance)))) "AlwaysSpawn" self 0)
        (Development|PrintString "Spawngalaxy")))
    (:then_1)))